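; Game instance that manages front-end menus, the loading screen and multiplayer session flow.
; A save-game check opens either the main menu or first-run options with a welcome message; most widgets are cached for reuse, while the server menu is recreated each time.
; Hosting creates a session ignoring the LAN flag, then opens Lobby as a listen server; events also join and destroy sessions.
; Failures route to DisplayErrorMessage, which, like both error-to-string helpers, is an empty stub.
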(event Custom|ShowMainMenu
  (bind _returnvalue (Game|GetPlayerController 0))
  ;[1 1 1] 메인 메뉴를 보여주고 마우스 커서를 표시
  (Utilities|IsValid (Variables|Widgets|GetMainMenuWB)
    (:Is%20Valid
      _)
    (:Is%20Not%20Valid
      (bind _returnvalue_2 (UserInterface|CreateWidget "/Game/UI/MainMenu/MainMenu.MainMenu_C" _returnvalue))
      (Variables|Widgets|SetMainMenuWB _returnvalue_2)))
  (UserInterface|Viewport|AddtoViewport (Variables|Widgets|GetMainMenuWB) 0)
  (Variables|/Script/Engine.PlayerController|SetbShowMouseCursor _returnvalue true))

(event Custom|ShowHostMenu
  ;[1 1 1] 호스트 메인 메뉴
  (Utilities|IsValid (Variables|Widgets|GetHostMenuWB)
    (:Is%20Valid
      _)
    (:Is%20Not%20Valid
      (bind _returnvalue (UserInterface|CreateWidget "/Game/UI/MainMenu/HostMenu.HostMenu_C" (Game|GetPlayerController 0)))
      (Variables|Widgets|SetHostMenuWB _returnvalue)))
  (UserInterface|Viewport|AddtoViewport (Variables|Widgets|GetHostMenuWB) 0))

(event Custom|ShowServerMenu
  ;[1 1 1] 서버 메뉴 보여주기 - 명령할때마다 새로 만듬
  (bind _returnvalue (UserInterface|CreateWidget "/Game/UI/MainMenu/ServerMenu.ServerMenu_C" (Game|GetPlayerController 0)))
  (UserInterface|Viewport|AddtoViewport _returnvalue 0))

(event Custom|ShowOptionsMenu
  ;[1 1 1] 옵션 메뉴를 보여줌
  (Utilities|IsValid (Variables|Widgets|GetOptionsMenuWB)
    (:Is%20Valid
      _)
    (:Is%20Not%20Valid
      (bind _returnvalue (UserInterface|CreateWidget "/Game/UI/MainMenu/OptionMenu.OptionMenu_C" (Game|GetPlayerController 0)))
      (Variables|Widgets|SetOptionsMenuWB _returnvalue)))
  (UserInterface|Viewport|AddtoViewport (Variables|Widgets|GetOptionsMenuWB) 0)
  (if (not (Variables|Default|GetCreatedSaveFile?))
    (Variables|/Game/UI/MainMenu/OptionMenu.OptionMenu_C|SetWelcomeMessageVis (Variables|Widgets|GetOptionsMenuWB) "Visible")))

(event Custom|LaunchLobby
  (params (NumberOfPlayers :type Integer) (EnableLan? :type Boolean) (ServerName :type Text))
  ;[1 1 1] 호스트 설정으로 로비 열기
  (Variables|ServerSettings|SetMaxPlayers NumberOfPlayers)
  (Variables|ServerSettings|SetServerName ServerName)
  (CallFunction|ShowLoadingScreen)
  (|Session (Game|GetPlayerController 0) (Variables|ServerSettings|GetMaxPlayers) false
    (:OnSuccess
      (Game|OpenLevel(byName) "Lobby" true "listen"))
    (:OnFailure
      (Utilities|DisplayErrorMessage "Failed To Create Session. Please Try Again"))))

(event Custom|ShowLoadingScreen
  ;[1 1 1] 요구시 로딩 스크린을 출력
  (Utilities|IsValid (Variables|Widgets|GetLoadingScreenWB)
    (:Is%20Valid
      _)
    (:Is%20Not%20Valid
      (bind _returnvalue (UserInterface|CreateWidget "/Game/UI/AllLevels/LoadingScreen.LoadingScreen_C" (Game|GetPlayerController 0)))
      (Variables|Widgets|SetLoadingScreenWB _returnvalue)))
  (UserInterface|Viewport|AddtoViewport (Variables|Widgets|GetLoadingScreenWB) 0))

(event Custom|JoinServer
  (params (SessionToJoin :type Blueprint%20Session%20Result%20Structure))
  ;[1 1 1] 서버 접속 - 서버 메뉴 불러오기.
  (CallFunction|ShowLoadingScreen)
  (|JoinSession (Game|GetPlayerController 0) SessionToJoin
    (:OnFailure
      (Utilities|DisplayErrorMessage "Failed To Join Session. Please Try Again"))))

(event Custom|DestroySessionCaller
  (params (PlayerController :type Player%20Controller%20Object%20Reference))
  ;[1 1 1] 호출시 세션 파기
  (|DestroySession PlayerController))

(event Custom|SaveGameCheck
  ;[1 1 1] 저장 파일 확인
  (bind _returnvalue (SaveGame|DoesSaveGameExist (Variables|Default|GetPlayerSettingsSave)))
  (if _returnvalue
    (CallFunction|ShowMainMenu)
    (Variables|Default|SetCreatedSaveFile? true)
    (else
      (CallFunction|ShowOptionsMenu)
      (Variables|/Script/Engine.PlayerController|SetbShowMouseCursor (Game|GetPlayerController 0) false))))

(event EventHandleNetworkError
  (params (FailureType :type ENetworkFailure%20Enum :default "NetDriverAlreadyExists") (bIsServer :type Boolean))
  ;[1 1 1] 네트워크 에러 처리 및 메시지 출력
  (if bIsServer
    _
    (else
      _))
  (Utilities|DisplayErrorMessage (CallFunction|NetErrortoString FailureType)))

(event EventHandleTravelError
  (params (FailureType :type ETravelFailure%20Enum :default "NoLevel"))
  ;[1 1 1] 트레블 에러 처리 및 메시지 출력
  (Utilities|DisplayErrorMessage (CallFunction|TravelErrortoString FailureType)))

(fn NetErrortoString
  (params (FailureType :type ENetworkFailure%20Enum :default "NetDriverAlreadyExists"))
  (return ""))

(fn TravelErrortoString
  (params (FailureType :type ETravelFailure%20Enum :default "NoLevel"))
  (return ""))